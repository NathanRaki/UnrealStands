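; StandPieces_BP is a stand that spawns puzzle-agnostic Piece_BP actors and spins them while something overlaps it.
; On BeginPlay it spawns pieces in a loop bounded by PiecesNumber, all 100 units above its own location, and stores them in the Pieces array.
; Any actor beginning or ending overlap calls the parent handler, then tells every stored piece to Rotate or StopRotate.
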(event EventBeginPlay
  (bind _returnvalue (Transformation|GetActorTransform))
  (for _index (range 0 (Variables|Default|GetpiecesNumber))
    (bind _returnvalue_2 (Game|SpawnActorfromClass "/Game/CreationEvaluation/Blueprints/Piece_BP.Piece_BP_C" (Math|Transform|MakeTransform (Math|Vector|MakeVector (.x (.location _returnvalue)) (.y (.location _returnvalue)) (+ (.z (.location _returnvalue)) 1e+02)) (.rotation _returnvalue) (.scale _returnvalue)) "AdjustIfPossibleButAlwaysSpawn" 0 0))
    (Utilities|Array|Add (Variables|Default|Getpieces) _returnvalue_2)))

(event Collision|EventActorBeginOverlap
  (params (OtherActor :type Actor%20Object%20Reference))
  (|CallParentFunction OtherActor)
  (for _array_element (Variables|Default|Getpieces)
    (Default|Rotate _array_element)))

(event EventTick
  (params (DeltaSeconds :type Float%20%28single-precision%29)))

(event Collision|EventActorEndOverlap
  (params (OtherActor :type Actor%20Object%20Reference))
  (|CallParentFunction OtherActor)
  (for _array_element (Variables|Default|Getpieces)
    (Default|StopRotate _array_element)))

(fn ConstructionScript
  (|CallParentFunction))