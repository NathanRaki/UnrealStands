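; StandFootball_BP is a stand actor that stages a repeatable soccer pass with a spawned footballer and ball.
; On BeginPlay it spawns a Footballer_BP above itself at a random yaw, then a Ballon_BP offset along that player's mesh vectors at a fixed height.
; An actor overlap plays the pass montage.
; On completion it destroys the ball, randomly re-yaws the player and loops back to spawn a new ball.
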(event EventBeginPlay
  (bind _returnvalue (Transformation|GetActorTransform))
  (bind _returnvalue_2 (Game|SpawnActorfromClass "/Game/CreationEvaluation/Blueprints/Footballer_BP.Footballer_BP_C" (Math|Transform|MakeTransform (Math|Vector|MakeVector (.x (.location _returnvalue)) (.y (.location _returnvalue)) (+ (.z (.location _returnvalue)) 1e+02)) (Math|Rotator|MakeRotator (.roll (.rotation _returnvalue)) (.pitch (.rotation _returnvalue)) (Math|Random|RandomFloatinRange -1.8e+02 1.8e+02)) (.scale _returnvalue)) "Undefined" 0 0))
  (bind _output_get (Variables|Default|SetFootballer _returnvalue_2))
  (bind _returnvalue_3 (Game|SpawnActorfromClass "/Game/CreationEvaluation/Blueprints/Ballon_BP.Ballon_BP_C" (Math|Transform|MakeTransform (Math|Vector|MakeVector (.x (+ (+ (.location (Transformation|GetActorTransform _output_get)) (* (Math|Vector|GetRightVector (Variables|/Script/Engine.Character|GetMesh _output_get)) 1e+02)) (* (Math|Vector|GetForwardVector (Variables|/Script/Engine.Character|GetMesh _output_get)) -3e+01))) (.y (+ (+ (.location (Transformation|GetActorTransform _output_get)) (* (Math|Vector|GetRightVector (Variables|/Script/Engine.Character|GetMesh _output_get)) 1e+02)) (* (Math|Vector|GetForwardVector (Variables|/Script/Engine.Character|GetMesh _output_get)) -3e+01))) 1.3e+02) "0, 0, 0" "0.700000,0.700000,0.700000") "AdjustIfPossibleButAlwaysSpawn" 0 0))
  (Variables|Default|SetBall _returnvalue_3))

(event Collision|EventActorBeginOverlap
  (params (OtherActor :type Actor%20Object%20Reference))
  (|CallParentFunction OtherActor)
  (Animation|Montage|PlayMontage (Variables|/Script/Engine.Character|GetMesh (Variables|Default|GetFootballer)) "/Game/CreationEvaluation/Imports/SoccerPass4UE4_Montage.SoccerPass4UE4_Montage"
    (:OnCompleted
      (Actor|DestroyActor (Variables|Default|GetBall))
      (Variables|Default|SetBall 0)
      (Transformation|SetActorRotation (Variables|Default|GetFootballer) (Math|Rotator|MakeRotator 0.0 0.0 (Math|Random|RandomFloatinRange -1.8e+02 1.8e+02)))
      (bind _returnvalue (Game|SpawnActorfromClass "/Game/CreationEvaluation/Blueprints/Ballon_BP.Ballon_BP_C" (Math|Transform|MakeTransform (Math|Vector|MakeVector (.x (+ (+ (.location (Transformation|GetActorTransform (stale EventBeginPlay _output_get))) (* (Math|Vector|GetRightVector (Variables|/Script/Engine.Character|GetMesh (stale EventBeginPlay _output_get))) 1e+02)) (* (Math|Vector|GetForwardVector (Variables|/Script/Engine.Character|GetMesh (stale EventBeginPlay _output_get))) -3e+01))) (.y (+ (+ (.location (Transformation|GetActorTransform (stale EventBeginPlay _output_get))) (* (Math|Vector|GetRightVector (Variables|/Script/Engine.Character|GetMesh (stale EventBeginPlay _output_get))) 1e+02)) (* (Math|Vector|GetForwardVector (Variables|/Script/Engine.Character|GetMesh (stale EventBeginPlay _output_get))) -3e+01))) 1.3e+02) "0, 0, 0" "0.700000,0.700000,0.700000") "AdjustIfPossibleButAlwaysSpawn" 0 0))
      (Variables|Default|SetBall _returnvalue))))

(event Collision|EventActorEndOverlap
  (params (OtherActor :type Actor%20Object%20Reference))
  (|CallParentFunction OtherActor))

(fn ConstructionScript
  (|CallParentFunction))