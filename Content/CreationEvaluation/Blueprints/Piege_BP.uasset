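; Piege_BP is a trap actor that rises 230 units above its starting position when triggered, then lowers back down.
; Trigger starts the rise and a 10-second delay, after which the movement reverses.
; Tick lerps the location between start and raised points over TimeToTrap without sweeping, pinning it at the top until the delay ends and stopping once it is back at the start.
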(event Custom|Trigger
  (Variables|Default|SetisTrapped true)
  (Variables|Default|SetElapsedTime 0.0)
  (Variables|Default|SetisMoving true)
  (Utilities|FlowControl|Delay 1e+01)
  (Variables|Default|SetisTrapped false)
  (Variables|Default|SetElapsedTime 0.0))

(event EventTick
  (params (DeltaSeconds :type Float%20%28single-precision%29))
  (if (Variables|Default|GetisMoving)
    (Variables|Default|SetElapsedTime (+ (Variables|Default|GetElapsedTime) DeltaSeconds))
    (if (Variables|Default|GetisTrapped)
      (Transformation|SetActorLocation (Math|Vector|Lerp(Vector) (Variables|Default|GetstartLocation) (Variables|Default|GetendLocation) (/ (Variables|Default|GetElapsedTime) (Variables|Default|GetTimeToTrap))) false false)
      (if (>= (Variables|Default|GetElapsedTime) (Variables|Default|GetTimeToTrap))
        (Transformation|SetActorLocation (Variables|Default|GetendLocation) false false))
      (else
        (Transformation|SetActorLocation (Math|Vector|Lerp(Vector) (Variables|Default|GetendLocation) (Variables|Default|GetstartLocation) (/ (Variables|Default|GetElapsedTime) (Variables|Default|GetTimeToTrap))) false false)
        (if (>= (Variables|Default|GetElapsedTime) (Variables|Default|GetTimeToTrap))
          (Transformation|SetActorLocation (Variables|Default|GetstartLocation) false false)
          (Variables|Default|SetisMoving false))))))

(event EventBeginPlay
  (bind _output_get (Variables|Default|SetstartLocation (Transformation|GetActorLocation)))
  (Variables|Default|SetendLocation (Math|Vector|MakeVector (.x _output_get) (.y _output_get) (+ (.z _output_get) 2.3e+02))))

(fn ConstructionScript)