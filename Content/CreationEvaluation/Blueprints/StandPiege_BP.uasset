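; StandPiege_BP is a trap stand actor that owns and arms a Piege_BP trap.
; On BeginPlay it spawns the trap at a fixed offset from itself with its own rotation, keeps a reference, and passes its TimeToTrap value to it.
; Any actor that begins overlapping the stand calls Trigger on that spawned trap.
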(event Collision|EventActorBeginOverlap
  (params (OtherActor :type Actor%20Object%20Reference))
  (|CallParentFunction OtherActor)
  (Default|Trigger (Variables|Default|GetPiege)))

(event EventBeginPlay
  (bind _returnvalue (Transformation|GetActorTransform))
  (bind _returnvalue_2 (Game|SpawnActorfromClass "/Game/CreationEvaluation/Blueprints/Piege_BP.Piege_BP_C" (Math|Transform|MakeTransform (+ (.location _returnvalue) "-370.000000, 0, 0") (.rotation _returnvalue) "1.093750,1.093750,1") "Undefined" 0 0))
  (bind _output_get (Variables|Default|SetPiege _returnvalue_2))
  (Variables|/Game/CreationEvaluation/Blueprints/Piege_BP.Piege_BP_C|SetTimeToTrap _output_get (Variables|Default|GettimeToTrap)))

(event Collision|EventActorEndOverlap
  (params (OtherActor :type Actor%20Object%20Reference))
  (|CallParentFunction OtherActor))

(fn ConstructionScript
  (|CallParentFunction))