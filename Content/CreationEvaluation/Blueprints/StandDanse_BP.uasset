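; StandDanse_BP is a stand actor that makes a dancing character perform while something overlaps it.
; On BeginPlay it spawns a DancingCharacter_BP 100 units above itself, with the stand's rotation and scale, and keeps a reference to it.
; Begin and end overlap call the parent handlers, then Dance and StopDance on that character, with no filter on the overlapping actor.
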(event EventBeginPlay
  (bind _returnvalue (Transformation|GetActorTransform))
  (bind _returnvalue_2 (Game|SpawnActorfromClass "/Game/CreationEvaluation/Blueprints/DancingCharacter_BP.DancingCharacter_BP_C" (Math|Transform|MakeTransform (Math|Vector|MakeVector (.x (.location _returnvalue)) (.y (.location _returnvalue)) (+ (.z (.location _returnvalue)) 1e+02)) (.rotation _returnvalue) (.scale _returnvalue)) "Undefined" 0 0))
  (Variables|Default|SetDancingCharacter _returnvalue_2))

(event Collision|EventActorBeginOverlap
  (params (OtherActor :type Actor%20Object%20Reference))
  (|CallParentFunction OtherActor)
  (Default|Dance (Variables|Default|GetDancingCharacter)))

(event Collision|EventActorEndOverlap
  (params (OtherActor :type Actor%20Object%20Reference))
  (|CallParentFunction OtherActor)
  (Default|StopDance (Variables|Default|GetDancingCharacter)))

(fn ConstructionScript
  (|CallParentFunction))