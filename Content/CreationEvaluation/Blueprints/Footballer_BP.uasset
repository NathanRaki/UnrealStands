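; Footballer actor that knocks a Ballon_BP ball away when it overlaps it.
; On BeginPlay, it attaches its Capsule to the mesh's ik_foot_r socket so the capsule follows the right foot.
; Any actor overlap with the ball applies a mass-independent impulse to the ball's Sphere, along the unnormalized footballer-to-ball vector, so strength scales with the distance between actor origins.
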(event EventBeginPlay
  (Transformation|AttachComponentToComponent (Variables|Default|GetCapsule) (Variables|Character|GetMesh) "ik_foot_r" "KeepRelative" "KeepRelative" "KeepRelative" true))

(event Collision|EventActorBeginOverlap
  (params (OtherActor :type Actor%20Object%20Reference))
  (bind _asballon_bp (Utilities|Casting|CastToBallon_BP OtherActor))
  (Physics|AddImpulse (Variables|/Game/CreationEvaluation/Blueprints/Ballon_BP.Ballon_BP_C|GetSphere _asballon_bp) (* (- (Transformation|GetActorLocation _asballon_bp) (Transformation|GetActorLocation)) 5e+01) "None" true))

(fn ConstructionScript)